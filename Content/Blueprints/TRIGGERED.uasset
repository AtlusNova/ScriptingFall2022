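; TRIGGERED is a trigger actor that awards score in the BouncyRoom game mode when another actor overlaps it.
; On begin overlap it casts the game mode to BouncyRoom, adds one point and spawns a sparks particle system at the overlapping actor's location.
; Enter and exit debug prints remain in the graph but are disconnected.
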(event `self.ReceiveBeginPlay`)

(event `self.ReceiveActorBeginOverlap`
  (params (OtherActor :type "Actor Object Reference"))
  (bind _asbouncy_room (cast `/Game/Blueprints/BouncyRoom` (`GameplayStatics.GetGameMode`)))
  (`/Game/Blueprints/BouncyRoom.AddScore` _asbouncy_room 1)
  (`NiagaraFunctionLibrary.SpawnSystemAtLocation` "/Game/Particles/SparksSystem.SparksSystem" (`self.K2_GetActorLocation` OtherActor)))

(event `self.ReceiveActorEndOverlap`
  (params (OtherActor :type "Actor Object Reference")))

(fn `UserConstructionScript`)