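; A player pawn that possesses itself on BeginPlay and launches its physics spheres when the click input is pressed.
; The click event calls Impulse, which adds the same fixed force to four sphere components along the combined world up and right vectors.
; The force goes through AddForce as a plain force, without acceleration change, despite the function's name.
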(event `InputAction|click`
  (params (Key :type "Key Structure"))
  (:`Pressed`
    (`self.Impulse` 70000.0)))

(event `self.ReceiveBeginPlay`
  (bind _returnvalue (`GameplayStatics.GetPlayerController` 0))
  (`Controller.Possess` _returnvalue self)
  (`self.EnableInput` _returnvalue))

(fn `Impulse`
  (params (Force :type "Float (double-precision)"))
  (bind _returnvalue (* (+ (`KismetMathLibrary.Vector_Up`) (`KismetMathLibrary.Vector_Right`)) Force))
  (`PrimitiveComponent.AddForce` (`self.Sphere1`) _returnvalue "None" false)
  (`PrimitiveComponent.AddForce` (`self.Sphere2`) _returnvalue "None" false)
  (`PrimitiveComponent.AddForce` (`self.Sphere3`) _returnvalue "None" false)
  (`PrimitiveComponent.AddForce` (`self.Sphere4`) _returnvalue "None" false))

(fn `UserConstructionScript`)