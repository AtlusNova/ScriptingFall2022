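; A sphere Blueprint that pushes itself upward when the click input action is pressed.
; BeginPlay enables input from player controller 0 and calls Possess on it with no pawn connected.
; Each press calls the Impulse function, which applies a one-off upward AddForce to the Sphere component, without acceleration change, and briefly prints a debug "Hello".
; Overlap, Tick and the construction script are empty.
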(event `InputAction|click`
  (params (Key :type "Key Structure"))
  (:`Pressed`
    (`self.Impulse` 1000.0)))

(event `self.ReceiveBeginPlay`
  (bind _returnvalue (`GameplayStatics.GetPlayerController` 0))
  (`Controller.Possess` _returnvalue null)
  (`self.EnableInput` _returnvalue))

(fn `Impulse`
  (params (Force :type "Float (double-precision)"))
  (`PrimitiveComponent.AddForce` (`self.Sphere`) (* (`KismetMathLibrary.Vector_Up`) Force) "None" false)
  (`KismetSystemLibrary.PrintText` "Hello" true true (struct :`G` 0.66 :`B` 1.0 :`A` 1.0) 0.1))

(fn `UserConstructionScript`)