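; Cube actor Blueprint that moves its static mesh steadily along world Z during play.
; Tick adds DeltaSeconds times Speed to the mesh's world Z without sweeping, keeping the motion frame-rate independent.
; The construction script and BeginPlay each print a "Salutations" debug greeting.
; Two disconnected frame-counter snippets, an older addition and an increment-operator version with a print, never run.
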(event `self.ReceiveBeginPlay`
  (`KismetSystemLibrary.PrintString` "Salutations"))

(event `self.ReceiveTick`
  (params (DeltaSeconds :type "Float (single-precision)"))
  (bind _staticmeshcomponent (`self.StaticMeshComponent`))
  (`SceneComponent.K2_SetWorldLocation` _staticmeshcomponent (`KismetMathLibrary.MakeVector` (.x (`SceneComponent.K2_GetComponentLocation` _staticmeshcomponent)) (.y (`SceneComponent.K2_GetComponentLocation` _staticmeshcomponent)) (+ (.z (`SceneComponent.K2_GetComponentLocation` _staticmeshcomponent)) (* DeltaSeconds (`self.Speed`)))) false false))

(fn `UserConstructionScript`
  (`KismetSystemLibrary.PrintString` "Salutations" true true (struct :`R` 1.0 :`B` 0.152277 :`A` 1.0)))